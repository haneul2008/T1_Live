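; Actor component that gives its owner health and a simple way to deal and receive damage.
; Hp starts at MaxHp on BeginPlay.
; CombatAttack forwards damage to the hit actor's CombatComponent, if it has one, through CombatHit.
; CombatHit clamps the reduced Hp, broadcasts the change, and fires an Hp-zero event when health runs out.
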(event `self.ReceiveBeginPlay`
  (set `self.Hp` (`self.MaxHp`)))

(fn `CombatAttack`
  (params (damage :type "Float (double-precision)") (hitActor :type "Actor Object Reference"))
  (bind _returnvalue (`Actor.GetComponentByClass` hitActor "CombatComponent_C"))
  (`/Engine/EditorBlueprintResources/StandardMacros.IsValid` _returnvalue
    (:`Is Valid`
      (`self.CombatHit` _returnvalue damage))))

(fn `CombatHit`
  (params (damage :type "Float (double-precision)"))
  (bind _output_get (set `self.Hp` (`KismetMathLibrary.FClamp` (- (`self.Hp`) damage) 0.0 (`self.MaxHp`))))
  (`self.OnChangedHp` _output_get (`self.MaxHp`))
  (if (<= (`self.Hp`) 0.0)
    (`self.OnHpZero`)))