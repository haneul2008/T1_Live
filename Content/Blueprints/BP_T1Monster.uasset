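; BP_T1Monster is a monster Blueprint that provides a melee-style attack hit check.
; AttackHitCheck sweeps a sphere forward from the actor's location, sized by AttackRange and AttackRadius, with a timed debug draw.
; A hit only prints the struck actor's name, with no damage applied.
; The event graph and construction script are empty, so nothing in this file calls the check.
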(event `self.ReceiveBeginPlay`)

(fn `AttackHitCheck`
  (bind _returnvalue (`self.K2_GetActorLocation`))
  (bind (_outhit _returnvalue_2) (`KismetSystemLibrary.SphereTraceSingle` :`Start` _returnvalue :`End` (+ _returnvalue (* (`self.GetActorForwardVector`) (`self.AttackRange`))) :`Radius` (`self.AttackRadius`) :`TraceChannel` "TraceTypeQuery4" :`DrawDebugType` "ForDuration" :`DrawTime` 0.5))
  (if _returnvalue_2
    (`KismetSystemLibrary.PrintString` (`KismetSystemLibrary.GetDisplayName` (`.HitActor` (`GameplayStatics.BreakHitResult` _outhit))))))

(fn `UserConstructionScript`)